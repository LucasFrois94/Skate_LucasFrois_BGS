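; BP_BaseItem is a collectible pickup, apparently a base class for items, that grants score in the skater game.
; When a BP_Skater overlaps its sphere, it adds its AddScore value to the GM_Skater game mode.
; It then spawns a Niagara blink effect and a coin sound at its location and destroys itself.
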(event OnComponentBeginOverlap(Sphere)
  (params (OverlappedComponent :type Primitive%20Component%20Object%20Reference) (OtherActor :type Actor%20Object%20Reference) (OtherComp :type Primitive%20Component%20Object%20Reference) (OtherBodyIndex :type Integer) (bFromSweep :type Boolean) (SweepResult :type Hit%20Result%20Structure%20%28by%20ref%29))
  (Utilities|Casting|CastToBP_Skater OtherActor)
  (CallFunction|AddonGM)
  (CallFunction|SpawnFX)
  (Actor|DestroyActor))

(fn ConstructionScript)

(fn AddonGM
  (bind _asgm_skater (Utilities|Casting|CastToGM_Skater (Game|GetGameMode)))
  (Default|AddScore _asgm_skater (Variables|Default|GetAddScore)))

(fn SpawnFX
  (Niagara|SpawnSystematLocation "/Game/BlinkAndDashVFX/VFX_Niagara/NS_Curse_Blink.NS_Curse_Blink" (Transformation|GetActorLocation))
  (Audio|SpawnSoundatLocation "/Game/Audio/MedievalCombatSounds/BONUS/wav/Coins_01_Cue.Coins_01_Cue" (Transformation|GetActorLocation) "0, 0, 0" 1.0 1.0 0.0 0 0))